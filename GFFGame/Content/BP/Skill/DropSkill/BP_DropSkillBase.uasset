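; Base dropped-skill pickup that looks up its skill in DT_Skill by enum and shows that skill's sprite.
; Player capsule overlap fills the first empty of two skill slots, spawns a follow-up actor, plays a sound and destroys the pickup.
; With both slots full, it spawns a skill-switch UI actor and flags the offered skill on the player.
; Tick polls overlaps through a Gate, clearing that offer and UI once the player leaves.
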(event OnComponentBeginOverlap(Cube)
  (params (OverlappedComponent :type Primitive%20Component%20Object%20Reference) (OtherActor :type Actor%20Object%20Reference) (OtherComp :type Primitive%20Component%20Object%20Reference) (OtherBodyIndex :type Integer) (bFromSweep :type Boolean) (SweepResult :type Hit%20Result%20Structure%20%28by%20ref%29))
  (bind _returnvalue (Transformation|GetActorLocation))
  (bind _asbp_player (Utilities|Casting|CastToBP_Player OtherActor))
  (if (== (Variables|/Script/Engine.Character|GetCapsuleComponent _asbp_player) OtherComp)
    (bind _output_get (Variables|Default|SetAs%20BP%20Player _asbp_player))
    (if (or (== (.Enum (Utilities|Struct|BreakS_Skill (Variables|/Game/BP/Skill/BP_Skill.BP_Skill_C|GetSkill (Variables|/Game/BP/Player/BP_Player.BP_Player_C|GetSTATE_SKILL_1 _output_get)))) 0) (== (.Enum (Utilities|Struct|BreakS_Skill (Variables|/Game/BP/Skill/BP_Skill.BP_Skill_C|GetSkill (Variables|/Game/BP/Player/BP_Player.BP_Player_C|GetSTATE_SKILL_2 _output_get)))) 0)) ; どちらかが空ならtrue
      ;[1 1 1] スキル1
      (if (== (.Enum (Utilities|Struct|BreakS_Skill (Variables|/Game/BP/Skill/BP_Skill.BP_Skill_C|GetSkill (Variables|/Game/BP/Player/BP_Player.BP_Player_C|GetSTATE_SKILL_1 _output_get)))) 0) ; スキル1が空なら
        (Variables|/Game/BP/Skill/BP_Skill.BP_Skill_C|SetSkill (Variables|/Game/BP/Player/BP_Player.BP_Player_C|GetSTATE_SKILL_1 _output_get) (Variables|Default|GetSkill))
        (Game|SpawnActorfromClass "/Game/BP/Skill/NewBlueprint1.NewBlueprint1_C" (Math|Transform|MakeTransform (Transformation|GetActorLocation) "0, 0, 0" "1.000000,1.000000,1.000000") "Undefined" "MultiplyWithRoot" 0 (Variables|Default|GetSkill) 0 :!label _label)
        (bind _ui_skillswitch (Variables|Default|GetUI_SkillSwitch)
          (:then
            (Actor|DestroyActor _ui_skillswitch))
          (:else
            _))
        (Actor|DestroyActor)
        (Audio|PlaySound2D "/Game/Sounds/SE/SE_Get.SE_Get" 1.0 1.0 0.0 0 0)
        (else
          ;[1 1 1] スキル2
          (if (== (.Enum (Utilities|Struct|BreakS_Skill (Variables|/Game/BP/Skill/BP_Skill.BP_Skill_C|GetSkill (Variables|/Game/BP/Player/BP_Player.BP_Player_C|GetSTATE_SKILL_2 _output_get)))) 0)
            (Variables|/Game/BP/Skill/BP_Skill.BP_Skill_C|SetSkill (Variables|/Game/BP/Player/BP_Player.BP_Player_C|GetSTATE_SKILL_2 _output_get) (Variables|Default|GetSkill))
            (goto _label))))
      (else
        (bind _returnvalue_2 (Game|SpawnActorfromClass "/Game/BP/Skill/NewBlueprint.NewBlueprint_C" (Math|Transform|MakeTransform (Math|Vector|MakeVector (.x _returnvalue) 1.0 (+ (.z _returnvalue) 128.0)) "0, 0, 0" "1.000000,1.000000,1.000000") "Undefined" "MultiplyWithRoot" 0 (Variables|Default|GetSkill) (Variables|Default|GetAs%20BP%20Player) 0))
        (Variables|Default|SetUI_SkillSwitch _returnvalue_2)
        (Variables|/Game/BP/Player/BP_Player.BP_Player_C|SetVALUE_GETSKILL? (Variables|Default|GetAs%20BP%20Player) true)
        (Variables|/Game/BP/Player/BP_Player.BP_Player_C|SetVALUE_DROPSKILL (Variables|Default|GetAs%20BP%20Player) (Variables|Default|GetSkill))))))

(event OnComponentEndOverlap(Box)
  (params (OverlappedComponent :type Primitive%20Component%20Object%20Reference) (OtherActor :type Actor%20Object%20Reference) (OtherComp :type Primitive%20Component%20Object%20Reference) (OtherBodyIndex :type Integer)))

(event EventBeginPlay
  (bind _returnvalue (Utilities|GetDataTableRow "/Game/BP/Player/DT_Skill.DT_Skill" (Utilities|String|StringToName (Utilities|String|EnumtoString (Variables|Default|GetSTATE_SKILL))))
    (:then
      (bind _output_get (Variables|Default|SetSkill _returnvalue))
      (Rendering|Components|Sprite|SetSprite (Variables|Default|GetRenderComponent) (.AsPaper%20Sprite (Utilities|Casting|CastToPaperSprite (Utilities|Struct|BreakSlateBrush (.Image (Utilities|Struct|BreakS_Skill _output_get)))))))))

(event EventTick
  (params (DeltaSeconds :type Float%20%28single-precision%29))
  (Variables|Default|SetNewVar false)
  (Utilities|FlowControl|Sequence
    (:then_0
      (goto _label Open))
    (:then_1
      (for _array_element (Collision|GetOverlappingActors 0 :!class /Script/Engine.Actor)
        (bind _asbp_player (Utilities|Casting|CastToBP_Player _array_element))
        (Variables|Default|SetAs%20BP%20Player _asbp_player)
        (Utilities|IsValid (Variables|Default|GetUI_SkillSwitch)
          (:Is%20Valid
            (Variables|Default|SetNewVar true)
            (goto _label Close))))
      (if (Variables|Default|GetNewVar)
        (goto _label Close)
        (else
          (Utilities|FlowControl|Gate true :!label _label
            (:Exit
              (bind _as_bp_player (Variables|Default|GetAs%20BP%20Player)
                (:then
                  (Variables|/Game/BP/Player/BP_Player.BP_Player_C|SetVALUE_GETSKILL? _as_bp_player false)
                  (Variables|/Game/BP/Player/BP_Player.BP_Player_C|SetVALUE_DROPSKILL _as_bp_player "")
                  (bind _ui_skillswitch (Variables|Default|GetUI_SkillSwitch)
                    (:then
                      (Actor|DestroyActor _ui_skillswitch))
                    (:else)))
                (:else)))))))))

(fn ConstructionScript)