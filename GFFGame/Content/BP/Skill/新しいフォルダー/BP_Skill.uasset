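; BP_Skill runs one player skill chosen by enum: Small Shot, Spawn Block, Slash, or an empty Whip Shot stub.
; Active stores the player and starts the skill, spawning its projectile, block, or slash actor with Niagara effect.
; A cooldown timer, set from CoolTime/60, lets Tick re-fire the skill while active.
; Tick also updates the Small Shot aim cursor and keeps Slash on the player, oriented by control yaw.
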(event Custom|DeActive
  (Variables|Default|SetIsActive? false))

(event Custom|Active
  (params (OtherActor :type Actor%20Object%20Reference))
  (Variables|Default|SetOther%20Actor OtherActor)
  (Variables|Default|SetIsActive? true)
  (CallFunction|SkillStart))

(event EventTick
  (params (DeltaSeconds :type Float%20%28single-precision%29))
  (Utilities|FlowControl|Sequence
    (:then_0
      (if (== (Utilities|Time|GetTimerRemainingTimebyHandle (Variables|Default|GetSkillCt)) -1.0)
        (Utilities|Struct|SetmembersinS_Skill (Variables|Default|GetSkill) false)
        (CallFunction|SkillStart)))
    (:then_1
      (switch Utilities|FlowControl|Switch|SwitchonE_Skill (.Enum (Utilities|Struct|BreakS_Skill (Variables|Default|GetSkill)))
        (:NewEnumerator1
          (|SmallShot_graph))
        (:NewEnumerator4
          (|CollapseGraph))))))

(fn ConstructionScript)

(fn SmallShot
  (bind _player (Variables|Default|GetPlayer))
  (bind _return (Default|CursorAngle _player 1.0))
  (bind _arrow1 (Variables|/Game/BP/Player/BP_Player.BP_Player_C|GetArrow1 _player))
  (bind _returnvalue (Transformation|GetSocketTransform _arrow1 "None" "RTS_World"))
  (bind (_location _rotation _scale) (Math|Transform|BreakTransform _returnvalue))
  (Game|SpawnActorfromClass "/Game/BP/Ammo/BP_SmallAmmo.BP_SmallAmmo_C" (Math|Transform|MakeTransform _location (Math|Rotator|SelectRotator _rotation (Math|Rotator|FindLookatRotation _location (+ _location _return)) (Utilities|Operators|EqualEqual :A _return)) _scale) "Undefined" "MultiplyWithRoot" 0 _player (.Damage (Utilities|Struct|BreakS_Skill (Variables|Default|GetSkill))) (Variables|Default|GetPlayer))
  (Audio|PlaySound2D "/Game/Sounds/SE/SE_Shot.SE_Shot" 1.0 1.0 0.0 0 0))

(fn SpawnBlock
  (bind _player (Variables|Default|GetPlayer))
  (bind _player_2 (Variables|Default|GetPlayer))
  (bind _player_3 (Variables|Default|GetPlayer))
  (bind _returnvalue (Transformation|GetActorLocation _player_2))
  (bind _return (Default|CursorAngle _player 1.0))
  (bind _return_2 (Default|CursorAngle _player_3 1.0))
  (if (> (Math|Float|Absolute(Float) (.x _return_2)) 0.8)
    (Game|SpawnActorfromClass "/Game/BP/Ammo/BP_SpawnBlock.BP_SpawnBlock_C" (Math|Transform|MakeTransform (+ _returnvalue (Math|Vector|MakeVector (* (Math|Float|Clamp(Float) (.x _return_2) -0.1 0.1) 2e+03) 0.0 0.0)) "0, 0, 0" "1.000000,1.000000,1.000000") "Undefined" "MultiplyWithRoot" 0 0)
    (elif (> (Math|Float|Absolute(Float) (.z _return)) 0.8)
      (Game|SpawnActorfromClass "/Game/BP/Ammo/BP_SpawnBlock.BP_SpawnBlock_C" (Math|Transform|MakeTransform (+ _returnvalue (Math|Vector|MakeVector 0.0 0.0 (* (Math|Float|Clamp(Float) (.z _return) -0.1 0.1) 2e+03))) "0, 0, 0" "1.000000,1.000000,1.000000") "Undefined" "MultiplyWithRoot" 0 0))))

(fn Slash
  (bind _player (Variables|Default|GetPlayer))
  (bind _returnvalue (Niagara|SpawnSystemAttached "/Game/Niagara/N_Slash.N_Slash" (Components|GetChildComponent (Variables|/Script/Engine.Character|GetCapsuleComponent (Variables|Default|GetPlayer)) 0) "None" "0, 0, 0" "0, 0, 0" "SnapToTarget" true))
  (Variables|Default|SetSlashNiagara _returnvalue)
  (bind _returnvalue_2 (Game|SpawnActorfromClass "/Game/BP/Ammo/BP_Slash.BP_Slash_C" (Math|Transform|MakeTransform "0, 0, 0" (Transformation|GetActorRotation _player) "1.000000,1.000000,1.000000") "Undefined" "MultiplyWithRoot" 0 _player))
  (Variables|Default|SetSlashActor _returnvalue_2)
  (Audio|PlaySound2D "/Game/Sounds/SE/SE_Slash.SE_Slash" 1.0 1.0 0.0 0 0))

(fn WhipShot)

(fn SkillStart
  (if (Variables|Default|GetIsActive?)
    (bind _asbp_player (Utilities|Casting|CastToBP_Player (Variables|Default|GetOther%20Actor)))
    (Variables|Default|SetPlayer _asbp_player)
    (if (not (Utilities|Struct|BreakS_Skill (Variables|Default|GetSkill)))
      (switch Utilities|FlowControl|Switch|SwitchonE_Skill (Utilities|Struct|BreakS_Skill (Variables|Default|GetSkill))
        (:NewEnumerator1
          (CallFunction|SmallShot))
        (:NewEnumerator3
          (CallFunction|SpawnBlock))
        (:NewEnumerator4
          (CallFunction|Slash))
        (:NewEnumerator5
          (CallFunction|WhipShot)))
      (Utilities|Struct|SetmembersinS_Skill (Variables|Default|GetSkill) true)
      (bind _returnvalue (Utilities|Time|SetTimerbyFunctionName 0 "SkillStart" (/ (Utilities|Struct|BreakS_Skill (Variables|Default|GetSkill)) 6e+01)))
      (Variables|Default|SetSkillCt _returnvalue))))

(fn SkillActive
  (Utilities|Struct|SetmembersinS_Skill (Variables|Default|GetSkill) false))