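; Actor component that gives its owning background actor a parallax scroll driven by the player camera.
; On BeginPlay it stores the owner's base location, then each Tick repositions the owner from the BP_Player camera's location.
; Horizontal X offset scales with the base Y as depth, Z follows at half the camera height, and Y stays fixed.
; An unconnected lerp-based smoothing chain remains in the graph but never runs.
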(event EventBeginPlay
  (bind _output_get (Variables|Default|SetLocationBase (Transformation|GetActorLocation (Components|GetOwner))))
  (Variables|Default|SetUI_Velocity _output_get))

(event EventTick
  (params (DeltaSeconds :type Float%20%28single-precision%29))
  (bind _locationbase (Variables|Default|GetLocationBase))
  (bind _asbp_player (Utilities|Casting|CastToBP_Player (Game|Player|GetPlayerPawn 0)))
  (Utilities|IsValid _asbp_player
    (:Is%20Valid
      (Transformation|SetActorLocation (Components|GetOwner) (Math|Vector|MakeVector (+ (* (.x (Transformation|GetSocketLocation (Variables|/Game/BP/Player/BP_Player.BP_Player_C|GetCamera _asbp_player) "None")) (.y _locationbase) -0.09) (.x _locationbase)) (.y _locationbase) (- (.z _locationbase) (* (.z (Transformation|GetSocketLocation (Variables|/Game/BP/Player/BP_Player.BP_Player_C|GetCamera _asbp_player) "None")) -0.5))) false false))))