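; Boss projectile actor that damages what its Cube collider overlaps and destroys itself after two seconds.
; Paper characters take Damage with a Niagara hit effect and sound; trigger actors take fixed damage.
; Character hits, tile maps and spawn blocks destroy the projectile.
; All hit handling sits inside a loop testing OtherActor against its own tags, a condition that cannot pass as wired.
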(event OnComponentBeginOverlap(Cube)
  (params (OverlappedComponent :type Primitive%20Component%20Object%20Reference) (OtherActor :type Actor%20Object%20Reference) (OtherComp :type Primitive%20Component%20Object%20Reference) (OtherBodyIndex :type Integer) (bFromSweep :type Boolean) (SweepResult :type Hit%20Result%20Structure%20%28by%20ref%29))
  (bind _returnvalue (Transformation|GetActorLocation))
  (bind _otheractor (Variables|Default|GetOtherActor)
    (:then
      (for _array_element (Variables|/Script/Engine.Actor|GetTags _otheractor)
        (if (not (Actor|ActorHasTag OtherActor _array_element))
          (bind _output_get (Variables|Default|SetHitActor OtherActor))
          (bind _aspaper_character (Utilities|Casting|CastToPaperCharacter _output_get)
            (:then
              (bind _returnvalue_2 (Niagara|SpawnSystematLocation "/Game/Niagara/N_AmmoHit.N_AmmoHit" (Math|Vector|Lerp(Vector) (Transformation|GetActorLocation _aspaper_character) _returnvalue 0.5)))
              (Niagara|SetNiagaraVariable(Vector3) _returnvalue_2 "Location" (Math|Vector|MakeVector (.X (Math|Vector|BreakVector (- (Transformation|GetActorLocation _aspaper_character) _returnvalue))) (.Y (Math|Vector|BreakVector (- (Transformation|GetActorLocation _aspaper_character) _returnvalue))) (/ (.Z (Math|Vector|BreakVector (- (Transformation|GetActorLocation _aspaper_character) _returnvalue))) 2.0)))
              (Game|Damage|ApplyDamage _aspaper_character (Math|Conversions|ToFloat(Integer) (Variables|Default|GetDamage)) (Game|GetInstigatorController) 0)
              (Audio|SpawnSound2D "/Game/Sounds/SE/SE_ShotHit.SE_ShotHit" 1.0 1.0 0.0 0)
              (Actor|DestroyActor))
            (:CastFailed
              (bind _asbp_trigger_base (Utilities|Casting|CastToBP_Trigger_Base (Variables|Default|GetHitActor))
                (:then
                  (Game|Damage|ApplyDamage _asbp_trigger_base 1.0 (Game|GetPlayerController 0) 0))
                (:CastFailed
                  (Utilities|FlowControl|Sequence
                    (:then_0
                      (Utilities|Casting|CastToPaperTileMapActor (Variables|Default|GetHitActor)))
                    (:then_2
                      (Utilities|Casting|CastToBP_SpawnBlock (Variables|Default|GetHitActor))))
                  (Actor|DestroyActor))))))))
    (:else)))

(event EventBeginPlay
  (Utilities|FlowControl|Delay 2.0)
  (Actor|DestroyActor))

(fn ConstructionScript)