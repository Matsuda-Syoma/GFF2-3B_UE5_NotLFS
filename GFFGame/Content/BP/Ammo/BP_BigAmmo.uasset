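; BP_BigAmmo is an ammo actor that destroys itself three seconds after spawning.
; Its Cube overlap handler is set up to spawn an N_AmmoHit effect midway between itself and an overlapped BP_Enemy_Base.
; The gating check compares OtherActor with itself for inequality, so the effect branch does not run as written.
; HitDamage is an empty stub and the Damage variable is unused, so it deals no damage.
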(event OnComponentBeginOverlap(Cube)
  (params (OverlappedComponent :type Primitive%20Component%20Object%20Reference) (OtherActor :type Actor%20Object%20Reference) (OtherComp :type Primitive%20Component%20Object%20Reference) (OtherBodyIndex :type Integer) (bFromSweep :type Boolean) (SweepResult :type Hit%20Result%20Structure%20%28by%20ref%29))
  (if (!= OtherActor (Variables|Default|GetOtherActor))
    (bind _asbp_enemy_base (Utilities|Casting|CastToBP_Enemy_Base OtherActor))
    (Niagara|SpawnSystematLocation "/Game/Niagara/N_AmmoHit.N_AmmoHit" (Math|Vector|Lerp(Vector) (Transformation|GetActorLocation _asbp_enemy_base) (Transformation|GetActorLocation) 0.5))))

(event EventBeginPlay
  (Utilities|FlowControl|Delay 3.0)
  (Actor|DestroyActor))

(fn ConstructionScript)