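; BP_SpawnBlock is a short-lived sprite actor that blinks at an increasing rate and destroys itself five seconds after BeginPlay.
; After a brief delay it starts a timeline, used as a repeating timer that restarts itself on Finished with an incrementing play rate.
; Each finish also drives a FlipFlop that alternates the sprite between opaque white and translucent black, so the blinking accelerates until removal.
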(event EventBeginPlay
  (bind _rendercomponent (Variables|Default|GetRenderComponent))
  (Utilities|FlowControl|Sequence
    (:then_0
      (Utilities|FlowControl|Delay 5.0)
      (Actor|DestroyActor))
    (:then_1
      (Utilities|FlowControl|Delay 0.75)
      (Timeline|タイムライン Play
        (:Finished
          (Utilities|FlowControl|Sequence
            (:then_0
              (Components|Timeline|SetPlayRate (Variables|Default|Getタイムライン) (Variables|Default|GetNew%20Rate))
              (Math|Float|IncrementFloat (Variables|Default|GetNew%20Rate)
                (:%20%20
                  (Timeline|タイムライン PlayFromStart))))
            (:then_1
              (Utilities|FlowControl|FlipFlop
                (:A
                  (Sprite|SetSpriteColor _rendercomponent "(R=1.000000,G=1.000000,B=1.000000,A=1.000000)"))
                (:B
                  (Sprite|SetSpriteColor _rendercomponent "(R=0.000000,G=0.000000,B=0.000000,A=0.666667)"))))))))))

(fn ConstructionScript)