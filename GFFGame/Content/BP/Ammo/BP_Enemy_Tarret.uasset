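; Enemy turret that continuously fires BP_SmallAmmo along a fixed angle, without aiming at the player.
; Tick spawns a projectile at the Shot1 component with ShotDamage, then uses the Active flag and a Delay to gate the cooldown, with CoolTime expressed in 60 fps frames.
; The shot sound plays in 2D only when the player is nearby.
; The construction script calls its parent and sets Shot1's world pitch from Angle.
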(event EventTick
  (params (DeltaSeconds :type Float%20%28single-precision%29))
  (bind _self self)
  (if (not (Variables|Default|GetActive))
    (Game|SpawnActorfromClass "/Game/BP/Ammo/BP_SmallAmmo.BP_SmallAmmo_C" (Transformation|GetSocketTransform (Variables|Default|GetShot1) "None" "RTS_World") "Undefined" "MultiplyWithRoot" 0 _self (Variables|Default|GetShotDamage) _self)
    (if (< (Math|Float|Absolute(Float) (Math|Vector|VectorLength (- (Transformation|GetActorLocation) (Transformation|GetActorLocation (Game|GetPlayerCharacter 0))))) 1.6e+03)
      (Audio|SpawnSound2D "/Game/Sounds/SE_EnemyShot.SE_EnemyShot" 1.0 1.0 0.0 0))
    (Variables|Default|SetActive true)
    (Utilities|FlowControl|Delay (/ (Variables|Default|GetCoolTime) 6e+01))
    (Variables|Default|SetActive false)))

(fn ConstructionScript
  (|CallParentFunction)
  (Transformation|SetWorldRotation (Variables|Default|GetShot1) (Math|Rotator|MakeRotator 0.0 (Variables|Default|GetAngle) 0.0) false false))