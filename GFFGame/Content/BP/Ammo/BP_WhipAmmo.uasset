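; Whip projectile that yanks a hit Paper character backward along the projectile's forward axis, destroying itself after two seconds if still alive.
; On Cube overlap, past a per-tag check, it zeroes the character's velocity and targets a spot 150 units back.
; A looped sphere trace steps that spot further back until clear, then teleports the character there and destroys the projectile.
; Tile maps and slip floors just destroy it.
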(event OnComponentBeginOverlap(Cube)
  (params (OverlappedComponent :type Primitive%20Component%20Object%20Reference) (OtherActor :type Actor%20Object%20Reference) (OtherComp :type Primitive%20Component%20Object%20Reference) (OtherBodyIndex :type Integer) (bFromSweep :type Boolean) (SweepResult :type Hit%20Result%20Structure%20%28by%20ref%29))
  (for _array_element (Variables|/Script/Engine.Actor|GetTags (Variables|Default|GetOtherActor))
    (if (not (Actor|ActorHasTag OtherActor _array_element))
      (bind _output_get (Variables|Default|SetHitActor OtherActor))
      (bind _aspaper_character (Utilities|Casting|CastToPaperCharacter _output_get)
        (:then
          (Variables|/Script/Engine.MovementComponent|SetVelocity (Variables|/Script/Engine.Character|GetCharacterMovement (.AsPaper%20Character (Utilities|Casting|CastToPaperCharacter (Variables|Default|GetOtherActor)))) "0, 0, 0")
          (bind _returnvalue (Collision|SphereTraceByChannel (- (- (Transformation|GetActorLocation _aspaper_character) (* (Math|Vector|GetForwardVector (Variables|Default|GetPaperSprite)) 1.5e+02)) (Variables|Default|GetLocationGap)) (- (- (Transformation|GetActorLocation _aspaper_character) (* (Math|Vector|GetForwardVector (Variables|Default|GetPaperSprite)) 1.5e+02)) (Variables|Default|GetLocationGap)) 5e+01 "TraceTypeQuery1" false 0 "None" :!label _label))
          (if _returnvalue
            (Variables|Default|SetLocationGap (- (Variables|Default|GetLocationGap) (* (Math|Vector|GetForwardVector (Variables|Default|GetPaperSprite)) -1e+01)))
            (goto _label)
            (else
              (Transformation|SetActorLocation (Variables|Default|GetOtherActor) (- (- (Transformation|GetActorLocation _aspaper_character) (* (Math|Vector|GetForwardVector (Variables|Default|GetPaperSprite)) 1.5e+02)) (Variables|Default|GetLocationGap)) false false)
              (Variables|Default|SetLocationGap "0, 0, 0")
              (Actor|DestroyActor))))
        (:CastFailed
          (Utilities|FlowControl|Sequence
            (:then_0
              (Utilities|Casting|CastToPaperTileMapActor (Variables|Default|GetHitActor)))
            (:then_1
              (Utilities|Casting|CastToBP_SlipFloor (Variables|Default|GetHitActor))))
          (Actor|DestroyActor))))))

(event EventBeginPlay
  (Utilities|FlowControl|Delay 2.0)
  (Actor|DestroyActor))

(fn ConstructionScript)