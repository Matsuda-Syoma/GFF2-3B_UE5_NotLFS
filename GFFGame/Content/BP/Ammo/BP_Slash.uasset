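; BP_Slash is a short-lived slash attack hitbox that destroys itself a quarter second after spawning.
; Box overlaps with an enemy's capsule apply its Damage, play a slash sound, and spawn a Niagara hit effect near the enemy, with a direction offset passed to it.
; Overlapped BP_Trigger_Base actors instead receive one point of damage, with the slash as causer.
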(event OnComponentBeginOverlap(Box)
  (params (OverlappedComponent :type Primitive%20Component%20Object%20Reference) (OtherActor :type Actor%20Object%20Reference) (OtherComp :type Primitive%20Component%20Object%20Reference) (OtherBodyIndex :type Integer) (bFromSweep :type Boolean) (SweepResult :type Hit%20Result%20Structure%20%28by%20ref%29))
  (bind _returnvalue (Transformation|GetActorLocation))
  (if true
    (bind _asbp_enemy_base (Utilities|Casting|CastToBP_Enemy_Base OtherActor)
      (:then
        (if (== (Variables|/Script/Engine.Character|GetCapsuleComponent _asbp_enemy_base) OtherComp)
          (bind _returnvalue_2 (Niagara|SpawnSystematLocation "/Game/Niagara/N_AmmoHit.N_AmmoHit" (Math|Vector|Lerp(Vector) (Transformation|GetActorLocation _asbp_enemy_base) _returnvalue 0.1)))
          (Niagara|SetNiagaraVariable(Vector3) _returnvalue_2 "Location" (Math|Vector|MakeVector (.X (Math|Vector|BreakVector (- (Transformation|GetActorLocation _asbp_enemy_base) _returnvalue))) (.Y (Math|Vector|BreakVector (- (Transformation|GetActorLocation _asbp_enemy_base) _returnvalue))) (/ (.Z (Math|Vector|BreakVector (- (Transformation|GetActorLocation _asbp_enemy_base) _returnvalue))) 2.0)))
          (Game|Damage|ApplyDamage _asbp_enemy_base (Math|Conversions|ToFloat(Integer) (Variables|Default|GetDamage)) (Game|GetInstigatorController) 0)
          (Audio|SpawnSound2D "/Game/Sounds/SE/SE_SlashHit.SE_SlashHit" 1.0 1.0 0.0 0)))
      (:CastFailed
        (bind _asbp_trigger_base (Utilities|Casting|CastToBP_Trigger_Base OtherActor))
        (Game|Damage|ApplyDamage _asbp_trigger_base 1.0 (Game|GetInstigatorController) self)))))

(event EventBeginPlay
  (Variables|Default|SetActive true)
  (Utilities|FlowControl|Delay 0.25)
  (Variables|Default|SetActive false)
  (Actor|DestroyActor))

(fn ConstructionScript)