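; Small ammo projectile that homes in on an optional target and destroys itself two seconds after spawning.
; On overlap, its hit branch damages a Paper character with an impact Niagara effect and sound, then destroys the projectile.
; That branch is gated by testing the other actor against its own tags, so ordinary tags never pass.
; Handling for triggers, tilemaps, slip floors and spawn blocks is disconnected.
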(event OnComponentBeginOverlap(Cube)
  (params (OverlappedComponent :type Primitive%20Component%20Object%20Reference) (OtherActor :type Actor%20Object%20Reference) (OtherComp :type Primitive%20Component%20Object%20Reference) (OtherBodyIndex :type Integer) (bFromSweep :type Boolean) (SweepResult :type Hit%20Result%20Structure%20%28by%20ref%29))
  (bind _returnvalue (Transformation|GetActorLocation))
  (bind _otheractor (Variables|Default|GetOtherActor)
    (:then
      (for _array_element (Variables|/Script/Engine.Actor|GetTags _otheractor)
        (if (not (Actor|ActorHasTag OtherActor _array_element))
          (bind _output_get (Variables|Default|SetHitActor OtherActor))
          (bind _aspaper_character (Utilities|Casting|CastToPaperCharacter _output_get))
          (bind _returnvalue_2 (Niagara|SpawnSystematLocation "/Game/Niagara/N_AmmoHit.N_AmmoHit" (Math|Vector|Lerp(Vector) (Transformation|GetActorLocation _aspaper_character) _returnvalue 0.5)))
          (Niagara|SetNiagaraVariable(Vector3) _returnvalue_2 "Location" (Math|Vector|MakeVector (.X (Math|Vector|BreakVector (- (Transformation|GetActorLocation _aspaper_character) _returnvalue))) (.Y (Math|Vector|BreakVector (- (Transformation|GetActorLocation _aspaper_character) _returnvalue))) (/ (.Z (Math|Vector|BreakVector (- (Transformation|GetActorLocation _aspaper_character) _returnvalue))) 2.0)))
          (Game|Damage|ApplyDamage _aspaper_character (Math|Conversions|ToFloat(Integer) (Variables|Default|GetDamage)) (Game|GetInstigatorController) 0)
          (Audio|SpawnSound2D "/Game/Sounds/SE/SE_ShotHit.SE_ShotHit" 1.0 1.0 0.0 0)
          (Actor|DestroyActor))))
    (:else)))

(event EventBeginPlay
  (bind _projectilemovement (Variables|Default|GetProjectileMovement))
  (Utilities|FlowControl|Sequence
    (:then_0
      (Variables|Default|GetHomingTarget
        (:then
          (Variables|/Script/Engine.ProjectileMovementComponent|SetbIsHomingProjectile _projectilemovement true)
          (bind _returnvalue (AddComponent|AddSceneComponent (Variables|Default|GetHomingTarget) false))
          (Variables|/Script/Engine.ProjectileMovementComponent|SetHomingTargetComponent _projectilemovement _returnvalue)
          (Variables|/Script/Engine.ProjectileMovementComponent|SetHomingAccelerationMagnitude _projectilemovement 2e+04))
        (:else)))
    (:then_1
      (Utilities|FlowControl|Delay 2.0)
      (Actor|DestroyActor))))

(fn ConstructionScript)