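; BP_SpawnEnemy is a spawner gimmick that periodically creates walking slime enemies inside its Box volume.
; A looping five-second timer started on BeginPlay calls SpawnAIFromClass at a random point within the Box bounds.
; A failed spawn increments Count and retries only at the threshold or above; below it, Count resets and a "consecutive failure" message prints, so as wired the retry is effectively never reached.
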(event Custom|Spawn
  (bind _box (Variables|Default|GetBox))
  (bind (_origin _boxextent) (Collision|GetComponentBounds _box))
  (bind _returnvalue (AI|SpawnAIFromClass "/Game/BP/Enemy/BP_Enemy_WalkSlime.BP_Enemy_WalkSlime_C" 0 (Math|Random|RandomPointinBoundingBox _origin _boxextent) "0, 0, 0" false 0 :!label _label))
  (Utilities|IsValid _returnvalue
    (:Is%20Not%20Valid
      (bind _result (Math|Float|IncrementFloat (Variables|Default|GetCount))
        (:%20%20
          (if (>= _result 3e+01)
            (goto _label)
            (else
              (Variables|Default|SetCount 0.0)
              (Development|PrintString "連続失敗" true true "(R=1.000000,G=0.071741,B=0.000000,A=1.000000)"))))))))

(event EventBeginPlay
  (Utilities|Time|SetTimerbyEvent (delegate Custom|Spawn) 5.0 true))

(fn ConstructionScript)