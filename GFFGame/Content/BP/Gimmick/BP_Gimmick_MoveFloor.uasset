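; A 2D moving floor gimmick that travels horizontally and vertically once activated, built on a parent gimmick's Active event.
; Two timelines, MoveX and MoveY, play at MoveSpeed, their Alpha acting as a frame-time-scaled velocity for local X and Z offsets, multiplied by speed and per-axis length.
; The construction script widens the floor to FloorNum segments by adding evenly spaced child actors along X, matching the sprite's scale.
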(event EventActive
  (|CallParentFunction)
  (Components|Timeline|SetPlayRate (Variables|Default|GetMoveX) (Variables|Default|GetMoveSpeed))
  (Components|Timeline|SetPlayRate (Variables|Default|GetMoveY) (Variables|Default|GetMoveSpeed))
  (Utilities|FlowControl|Sequence
    (:then_0
      (bind _alpha (Timeline|MoveX Play)
        (:Update
          (Transformation|AddActorLocalOffset (Math|Vector|MakeVector (* (* (Utilities|Time|GetWorldDeltaSeconds) _alpha) (* (Variables|Default|GetMoveSpeed) 1e+02 (Variables|Default|GetMoveLengthX))) 0.0 0.0) false false))))
    (:then_1
      (bind _alpha_2 (Timeline|MoveY Play)
        (:Update
          (Transformation|AddActorLocalOffset (Math|Vector|MakeVector 0.0 0.0 (* (* (Utilities|Time|GetWorldDeltaSeconds) _alpha_2) (* (Variables|Default|GetMoveSpeed) 1e+02 (Variables|Default|GetMoveLengthY)))) false false))))))

(fn ConstructionScript
  (|CallParentFunction)
  (for _index (range 1 (- (Variables|Default|GetFloorNum) 1))
    (AddComponent|AddChildActorComponent false (Math|Transform|MakeTransform (Math|Vector|MakeVector (* _index 1e+02) 0.0 0.0) "0, 0, 0" (Variables|/Script/Engine.SceneComponent|GetRelativeScale3D (Variables|Default|GetPaperSprite))))))