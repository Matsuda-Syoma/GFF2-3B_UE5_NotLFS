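; Main game mode that runs score, countdown, pause and hit-stop for gameplay levels.
; BeginPlay creates the game HUD and a looping one-second timer that, at zero outside the "tyuto" level, fades out and opens the result map.
; KeepData and LoadData pass score, timer and two player skills through the GameInstance, retrying next tick until skills exist.
; Hit-stop freezes two actors via CustomTimeDilation with camera shake; pausing zeroes global time dilation.
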(event Custom|AddDataScore
  (params (Score :type Integer))
  (bind _output_get (Variables|Default|SetDataScore (+ (Variables|Default|GetDataScore) Score)))
  (Variables|/Game/UI/Game/UI_Game.UI_Game_C|SetDataScore (Variables|Default|GetUI_Game) _output_get))

(event Custom|AddViewScore
  (params (Score :type Integer))
  (bind _ui_game (Variables|Default|GetUI_Game))
  (bind _output_get (Variables|Default|SetViewScore (+ (Variables|Default|GetViewScore) Score)))
  (Variables|/Game/UI/Game/UI_Game.UI_Game_C|SetViewScore _ui_game _output_get)
  (UserInterface|Animation|PlayAnimation _ui_game (Variables|/Game/UI/Game/UI_Game.UI_Game_C|GetAddScoreAnim _ui_game) 0.0 1 "Forward" 1.0 false))

(event Custom|HitStop
  (params (ターゲット :type Actor%20Object%20Reference) (ターゲット2 :type Actor%20Object%20Reference) (StopFlame :type Float%20%28double-precision%29))
  (CameraShakes|StartCameraShake (Game|GetPlayerCameraManager 0) "/Game/BP/Camera/CS_Player.CS_Player_C" 1.0 "CameraLocal" "0, 0, 0")
  (Variables|/Script/Engine.Actor|SetCustomTimeDilation ターゲット 0.0)
  (Variables|/Script/Engine.Actor|SetCustomTimeDilation ターゲット2 0.0)
  (Utilities|FlowControl|Delay (* StopFlame (Utilities|Time|GetWorldDeltaSeconds)))
  (Variables|/Script/Engine.Actor|SetCustomTimeDilation ターゲット 1.0)
  (Utilities|IsValid ターゲット2
    (:Is%20Valid
      (Variables|/Script/Engine.Actor|SetCustomTimeDilation ターゲット2 1.0))))

(event Custom|Result
  (bind _returnvalue (UserInterface|CreateWidget "/Game/UI/UI_Fade.UI_Fade_C"))
  (UserInterface|Viewport|AddtoViewport _returnvalue 0)
  (Components|Animation|PlayAnimation _returnvalue (Variables|/Game/UI/UI_Fade.UI_Fade_C|GetFadeAnim _returnvalue) 0.0
    (:Finished
      (CallFunction|KeepData (CallFunction|GetGameMode))
      (Game|OpenLevel(byObjectReference) "/Game/Maps/Result/ResultMap.ResultMap"))))

(event EventBeginPlay
  (|CollapseGraph))

(fn ConstructionScript)

(fn KeepData
  (bind _as_bp_player (Variables|Default|GetAs%20BP%20Player))
  (bind _state_skill_1 (Variables|/Game/BP/Player/BP_Player.BP_Player_C|GetSTATE_SKILL_1 _as_bp_player))
  (bind _state_skill_2 (Variables|/Game/BP/Player/BP_Player.BP_Player_C|GetSTATE_SKILL_2 _as_bp_player))
  (bind _skill (Variables|/Game/BP/Skill/BP_Skill.BP_Skill_C|GetSkill _state_skill_2))
  (bind _skill_2 (Variables|/Game/BP/Skill/BP_Skill.BP_Skill_C|GetSkill _state_skill_1))
  (bind _asbp_game_instance (Utilities|Casting|CastToBP_GameInstance (Game|GetGameInstance)))
  (Utilities|Struct|SetmembersinS_Skill _skill_2 false)
  (Variables|/Game/BP/BP_GameInstance.BP_GameInstance_C|SetSkill1 _asbp_game_instance _skill_2)
  (Utilities|Struct|SetmembersinS_Skill _skill false)
  (Variables|/Game/BP/BP_GameInstance.BP_GameInstance_C|SetSkill2 _asbp_game_instance _skill)
  (Variables|/Game/BP/BP_GameInstance.BP_GameInstance_C|SetScore _asbp_game_instance (Variables|Default|GetDataScore))
  (Variables|/Game/BP/BP_GameInstance.BP_GameInstance_C|SetTimer _asbp_game_instance (Variables|Default|GetTimer)))

(fn CountTimer
  (if (<= (Variables|Default|GetTimer) 0)
    (bind _returnvalue (Game|GetCurrentLevelName true))
    (if (Utilities|Enum|NotEqual(Enum) _returnvalue "tyuto")
      (Utilities|FlowControl|DoOnce false
        (:Completed
          (CallFunction|Result))))
    (else
      (Math|Integer|DecrementInt (Variables|Default|GetTimer)))))

(fn 新規関数
  (if (== (Variables|/Game/BP/BP_GameInstance.BP_GameInstance_C|GetTimer (CallFunction|GetGameInstance)) 0)
    (Variables|Default|SetTimer (Variables|Default|GetMaxTimer))
    (else
      (Development|PrintString "err" true true "(R=1.000000,G=0.000000,B=0.000000,A=1.000000)"))))

(fn TimerSet
  (Variables|Default|SetTimer (Variables|Default|GetMaxTimer)))

(event Custom|LoadPlayer
  (bind _asbp_game_instance (CallFunction|GetGameInstance))
  (if (!= (Variables|/Game/BP/Player/BP_Player.BP_Player_C|GetSTATE_SKILL_1 (Variables|Default|GetAs%20BP%20Player)) 0)
    (Variables|/Game/BP/Skill/BP_Skill.BP_Skill_C|SetSkill (Variables|/Game/BP/Player/BP_Player.BP_Player_C|GetSTATE_SKILL_1 (Variables|Default|GetAs%20BP%20Player)) (Variables|/Game/BP/BP_GameInstance.BP_GameInstance_C|GetSkill1 _asbp_game_instance))
    (Variables|/Game/BP/Skill/BP_Skill.BP_Skill_C|SetSkill (Variables|/Game/BP/Player/BP_Player.BP_Player_C|GetSTATE_SKILL_2 (Variables|Default|GetAs%20BP%20Player)) (Variables|/Game/BP/BP_GameInstance.BP_GameInstance_C|GetSkill2 _asbp_game_instance))
    (else
      (Utilities|FlowControl|DelayUntilNextTick)
      (CallFunction|LoadPlayer))))

(event Custom|PauseFlip
  (bind _as_bp_player (Variables|Default|GetAs%20BP%20Player))
  (Utilities|FlowControl|FlipFlop
    (:A
      (bind _returnvalue (UserInterface|CreateWidget "/Game/UI/Game/UI_Pause.UI_Pause_C"))
      (UserInterface|Viewport|AddtoViewport _returnvalue 0)
      (Variables|Default|Setpause true)
      (Utilities|Time|SetGlobalTimeDilation 0.0)
      (Variables|/Game/BP/Player/BP_Player.BP_Player_C|SetVALUE_ISCURSOR? _as_bp_player false)
      (bind _newvar (Variables|/Game/BP/Player/BP_Player.BP_Player_C|GetNewVar _as_bp_player)
        (:then
          (Widget|RemovefromParent _newvar)
          (Input|SetInputModeGameandUI (Game|GetPlayerController 0) 0 "DoNotLock" true false))
        (:else)))
    (:B
      (Widget|RemovefromParent _returnvalue)
      (Utilities|Time|SetGlobalTimeDilation 1.0)
      (Variables|Default|Setpause false))))

(event Custom|LoadData
  (bind _asbp_game_instance (CallFunction|GetGameInstance))
  (Utilities|FlowControl|Sequence
    (:then_0
      (bind _output_get (Variables|Default|SetDataScore (Variables|/Game/BP/BP_GameInstance.BP_GameInstance_C|GetScore _asbp_game_instance)))
      (bind _output_get_2 (Variables|Default|SetViewScore _output_get))
      (Variables|Default|SetTimer (Variables|/Game/BP/BP_GameInstance.BP_GameInstance_C|GetTimer _asbp_game_instance))
      (bind _output_get_3 (Variables|/Game/UI/Game/UI_Game.UI_Game_C|SetDataScore (Variables|Default|GetUI_Game) _output_get_2))
      (Variables|/Game/UI/Game/UI_Game.UI_Game_C|SetViewScore (Variables|Default|GetUI_Game) _output_get_3))
    (:then_1
      (if (!= (Variables|/Game/BP/Player/BP_Player.BP_Player_C|GetSTATE_SKILL_1 (Variables|Default|GetAs%20BP%20Player)) 0)
        (Variables|/Game/BP/Skill/BP_Skill.BP_Skill_C|SetSkill (Variables|/Game/BP/Player/BP_Player.BP_Player_C|GetSTATE_SKILL_1 (Variables|Default|GetAs%20BP%20Player)) (Variables|/Game/BP/BP_GameInstance.BP_GameInstance_C|GetSkill1 _asbp_game_instance))
        (Variables|/Game/BP/Skill/BP_Skill.BP_Skill_C|SetSkill (Variables|/Game/BP/Player/BP_Player.BP_Player_C|GetSTATE_SKILL_2 (Variables|Default|GetAs%20BP%20Player)) (Variables|/Game/BP/BP_GameInstance.BP_GameInstance_C|GetSkill2 _asbp_game_instance))
        (else
          (Utilities|FlowControl|DelayUntilNextTick)
          (CallFunction|LoadPlayer))))))