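; BP_Camera is a camera zone that pulls the player's orthographic camera to its box center and zooms out while the player is inside.
; Each tick it scans box overlaps for BP_Player and sets that player's CameraMove state accordingly.
; A 20-step tick counter, frame-rate dependent, drives location and ortho-width lerps up to 1.5x base width at fixed depth, reversing on exit.
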(event EventTick
  (params (DeltaSeconds :type Float%20%28single-precision%29))
  (bind _as_bp_player (Variables|Default|GetAs%20BP%20Player))
  (bind _as_bp_player_2 (Variables|Default|GetAs%20BP%20Player))
  (bind _cameracnt (Variables|Default|GetCameraCnt))
  (bind _box (Variables|Default|GetBox))
  (bind _returnvalue (Transformation|GetWorldLocation _box))
  (bind _baseorthowidth (Variables|/Game/BP/Player/BP_Player.BP_Player_C|GetBaseOrthoWidth _as_bp_player))
  (Variables|Default|SetInPlayer? false)
  (Variables|/Game/BP/Player/BP_Player.BP_Player_C|SetCameraMove (Variables|Default|GetAs%20BP%20Player) "NewEnumerator0")
  (bind _array_element (Utilities|Array|ForEachLoopwithBreak (Collision|GetOverlappingActors (Variables|Default|GetBox) 0 :!class /Script/Engine.PrimitiveComponent) :!label _label)
    (:LoopBody
      (if (== _array_element (Variables|Default|GetAs%20BP%20Player))
        (Variables|Default|SetInPlayer? true)
        (Variables|/Game/BP/Player/BP_Player.BP_Player_C|SetCameraMove (Variables|Default|GetAs%20BP%20Player) "NewEnumerator1")
        (goto _label Break)))
    (:Completed
      (if (Variables|Default|GetInPlayer?)
        (if (< _cameracnt 20)
          (Math|Integer|IncrementInt (Variables|Default|GetCameraCnt)
            (:%20%20
              _)))
        (Transformation|SetWorldLocation (Variables|/Game/BP/Player/BP_Player.BP_Player_C|GetCamera _as_bp_player_2) (Math|Vector|Lerp(Vector) (Transformation|GetWorldLocation (Variables|/Game/BP/Player/BP_Player.BP_Player_C|GetScene _as_bp_player_2)) (Math|Vector|MakeVector (.x _returnvalue) 3e+02 (.z _returnvalue)) (/ (Math|Conversions|ToFloat(Integer) (Variables|Default|GetCameraCnt)) 2e+01)) false false :!label _label_2)
        (Class|CameraComponent|SetOrthoWidth (Variables|/Game/BP/Player/BP_Player.BP_Player_C|GetCamera _as_bp_player) (Math|Float|Lerp _baseorthowidth (* _baseorthowidth 1.5) (/ (Math|Conversions|ToFloat(Integer) (Variables|Default|GetCameraCnt)) 2e+01)))
        (elif (> _cameracnt 0)
          (Math|Integer|DecrementInt (Variables|Default|GetCameraCnt)
            (:%20%20
              (goto _label_2))))))))

(event EventBeginPlay
  (bind _asbp_player (Utilities|Casting|CastToBP_Player (Game|GetPlayerCharacter 0)))
  (Variables|Default|SetAs%20BP%20Player _asbp_player))

(fn ConstructionScript)