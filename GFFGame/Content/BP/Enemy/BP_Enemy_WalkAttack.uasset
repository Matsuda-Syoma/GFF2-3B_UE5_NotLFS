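; Walking enemy Blueprint that patrols back and forth while firing small projectiles.
; Tick drives forward movement at MoveSpeed and, through a Delay, spawns BP_SmallAmmo at its own transform about every two seconds.
; It flips 180 degrees when the capsule hits anything but the player, or, with Revese enabled, when an arrow-aimed line trace finds nothing, like an edge check.
; HitDamage is an empty stub.
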(event OnComponentHit(CapsuleComponent)
  (params (HitComponent :type Primitive%20Component%20Object%20Reference) (OtherActor :type Actor%20Object%20Reference) (OtherComp :type Primitive%20Component%20Object%20Reference) (NormalImpulse :type Vector :default "0, 0, 0") (Hit :type Hit%20Result%20Structure%20%28by%20ref%29))
  (Utilities|Casting|CastToBP_Player OtherActor
    (:CastFailed
      (Transformation|SetActorRotation (Math|Rotator|CombineRotators (Transformation|GetActorRotation) "0.000000,180.000000,0.000000")))))

(event Custom|Shoot
  (bind _self self)
  (Game|SpawnActorfromClass "/Game/BP/Ammo/BP_SmallAmmo.BP_SmallAmmo_C" (Math|Transform|MakeTransform (Transformation|GetActorLocation) (Transformation|GetActorRotation) "1.000000,1.000000,1.000000") "Undefined" "MultiplyWithRoot" 0 _self 1 _self))

(event EventTick
  (params (DeltaSeconds :type Float%20%28single-precision%29))
  (bind _arrow1 (Variables|Default|GetArrow1))
  (bind _returnvalue (Transformation|GetSocketLocation _arrow1 "None"))
  (Utilities|FlowControl|Sequence
    (:then_0
      (Pawn|Input|AddMovementInput (Transformation|GetActorForwardVector) (Variables|Default|GetMoveSpeed) false)
      (bind _returnvalue_2 (Collision|LineTraceByChannel _returnvalue (+ _returnvalue (* (Math|Vector|GetForwardVector _arrow1) 1e+02)) "TraceTypeQuery1" false 0 "None"))
      (if (Variables|Default|GetRevese)
        (if (not _returnvalue_2)
          (Transformation|SetActorRotation (Math|Rotator|CombineRotators (Transformation|GetActorRotation) "0.000000,180.000000,0.000000")))))
    (:then_1
      (Utilities|FlowControl|Delay 2.0)
      (CallFunction|Shoot))))

(event EventHitDamage
  (params (Damage :type Integer)))

(fn ConstructionScript
  (|CallParentFunction))