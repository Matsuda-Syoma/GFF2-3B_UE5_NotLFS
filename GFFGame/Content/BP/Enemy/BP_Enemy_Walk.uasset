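; BP_Enemy_Walk is a walking enemy that constantly moves forward and turns around at obstacles, leaving damage handling to its parent class.
; Each tick it traces a short visibility line along Arrow1 and, when Reverse is enabled, flips 180 degrees if nothing is hit, apparently to detect ledges.
; Capsule hits against anything other than BP_Player also flip its rotation.
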(event OnComponentHit(CapsuleComponent)
  (params (HitComponent :type Primitive%20Component%20Object%20Reference) (OtherActor :type Actor%20Object%20Reference) (OtherComp :type Primitive%20Component%20Object%20Reference) (NormalImpulse :type Vector :default "0, 0, 0") (Hit :type Hit%20Result%20Structure%20%28by%20ref%29))
  (Utilities|Casting|CastToBP_Player OtherActor
    (:CastFailed
      (Transformation|SetActorRotation (Math|Rotator|CombineRotators (Transformation|GetActorRotation) "0.000000,180.000000,0.000000")))))

(event EventTick
  (params (DeltaSeconds :type Float%20%28single-precision%29))
  (bind _arrow1 (Variables|Default|GetArrow1))
  (bind _returnvalue (Transformation|GetSocketLocation _arrow1 "None"))
  (Pawn|Input|AddMovementInput (Transformation|GetActorForwardVector) 1.0 false)
  (bind _returnvalue_2 (Collision|LineTraceByChannel _returnvalue (+ _returnvalue (* (Math|Vector|GetForwardVector _arrow1) 1e+02)) "TraceTypeQuery1" false 0 "None"))
  (if (Variables|Default|GetReverse)
    (if (not _returnvalue_2)
      (Transformation|SetActorRotation (Math|Rotator|CombineRotators (Transformation|GetActorRotation) "0.000000,180.000000,0.000000")))))

(event Game|Damage|EventAnyDamage
  (params (Damage :type Float%20%28single-precision%29) (DamageType :type Damage%20Type%20Object%20Reference) (InstigatedBy :type Controller%20Object%20Reference) (DamageCauser :type Actor%20Object%20Reference))
  (|CallParentFunction Damage DamageType InstigatedBy DamageCauser))

(fn ConstructionScript
  (|CallParentFunction))