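; Side-scrolling enemy that walks forward, turns around on hitting anything but the player, and lunges at the player on detection.
; When Reverse is set, it also turns whenever the Arrow1 line trace finds nothing.
; Search overlap pauses it briefly, then a per-frame delayed loop drives X/Z velocity toward the player's captured direction, with capsule collision temporarily overlap-only.
; Damage goes to the parent; contact damage is disconnected.
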(event OnComponentBeginOverlap(search)
  (params (OverlappedComponent :type Primitive%20Component%20Object%20Reference) (OtherActor :type Actor%20Object%20Reference) (OtherComp :type Primitive%20Component%20Object%20Reference) (OtherBodyIndex :type Integer) (bFromSweep :type Boolean) (SweepResult :type Hit%20Result%20Structure%20%28by%20ref%29))
  (bind _asbp_player (Utilities|Casting|CastToBP_Player OtherActor))
  (Variables|Default|SetNewVar_0 (Math|Vector|ClampVectorSize (- (Transformation|GetActorLocation _asbp_player) (Transformation|GetActorLocation)) 0.0 7e+01))
  (Pawn|Components|CharacterMovement|DisableMovement (Variables|Character|GetCharacterMovement))
  (Utilities|FlowControl|Delay 0.5)
  (Development|PrintString "Hello")
  (Pawn|Components|CharacterMovement|SetMovementMode (Variables|Character|GetCharacterMovement) "MOVE_Falling" 0) ; Movementを落下状態にする
  (Collision|SetCollisionProfileName (Variables|Default|GetCapsuleComponent) "OverlapOnlyPawn" true :!class /Script/Engine.PrimitiveComponent)
  ;[1 1 1] 毎フレーム数指定された分呼び出す
  (Utilities|WhileLoopwithDelay 0.0 (< (Variables|Default|GetCOUNT%20DA%20FLAME) (Variables|Default|GetSTATE%20DA%20FLAME))
    (:LoopBody
      (if (!= (Class|Actor|GetActorTimeDilation) 0.0)
        (Math|Integer|IncrementInt (Variables|Default|GetCOUNT%20DA%20FLAME) ; 呼び出されたら+1する
          (:%20%20
            (Variables|/Script/Engine.MovementComponent|SetVelocity (Variables|Character|GetCharacterMovement) (Math|Vector|MakeVector (.X (Math|Vector|BreakVector (* (* (Utilities|Time|GetWorldDeltaSeconds) (Variables|Default|GetNewVar_0)) (Variables|Default|GetDA_RANGE)))) 0.0 (.Z (Math|Vector|BreakVector (* (* (Utilities|Time|GetWorldDeltaSeconds) (Variables|Default|GetNewVar_0)) (Variables|Default|GetDA_RANGE)))))) ; カーソル*n分プレイヤーを動かす
          ))))
    (:Completed
      ;[1 1 1] ぬけたらプレイヤーの動きを止める
      (Variables|Default|SetCOUNT%20DA%20FLAME 0)
      (Variables|/Script/Engine.MovementComponent|SetVelocity (Variables|Character|GetCharacterMovement) (Math|Vector|MakeVector 0.0 0.0 0.0))
      (Collision|SetCollisionProfileName (Variables|Default|GetCapsuleComponent) "Pawn" true :!class /Script/Engine.PrimitiveComponent)
      (Utilities|FlowControl|Delay 1.0))))

(event OnComponentHit(CapsuleComponent)
  (params (HitComponent :type Primitive%20Component%20Object%20Reference) (OtherActor :type Actor%20Object%20Reference) (OtherComp :type Primitive%20Component%20Object%20Reference) (NormalImpulse :type Vector :default "0, 0, 0") (Hit :type Hit%20Result%20Structure%20%28by%20ref%29))
  (Utilities|Casting|CastToBP_Player OtherActor
    (:CastFailed
      (Transformation|SetActorRotation (Math|Rotator|CombineRotators (Transformation|GetActorRotation) "0.000000,180.000000,0.000000")))))

(event OnComponentBeginOverlap(CapsuleComponent)
  (params (OverlappedComponent :type Primitive%20Component%20Object%20Reference) (OtherActor :type Actor%20Object%20Reference) (OtherComp :type Primitive%20Component%20Object%20Reference) (OtherBodyIndex :type Integer) (bFromSweep :type Boolean) (SweepResult :type Hit%20Result%20Structure%20%28by%20ref%29)))

(event EventTick
  (params (DeltaSeconds :type Float%20%28single-precision%29))
  (bind _arrow1 (Variables|コンポーネント|GetArrow1))
  (bind _returnvalue (Transformation|GetSocketLocation _arrow1 "None"))
  (Pawn|Input|AddMovementInput (Transformation|GetActorForwardVector) 1.0 false)
  (bind _returnvalue_2 (Collision|LineTraceByChannel _returnvalue (+ _returnvalue (* (Math|Vector|GetForwardVector _arrow1) 1e+02)) "TraceTypeQuery1" false 0 "None"))
  (if (Variables|Default|GetReverse)
    (if (not _returnvalue_2)
      (Transformation|SetActorRotation (Math|Rotator|CombineRotators (Transformation|GetActorRotation) "0.000000,180.000000,0.000000")))))

(event Game|Damage|EventAnyDamage
  (params (Damage :type Float%20%28single-precision%29) (DamageType :type Damage%20Type%20Object%20Reference) (InstigatedBy :type Controller%20Object%20Reference) (DamageCauser :type Actor%20Object%20Reference))
  (|CallParentFunction Damage DamageType InstigatedBy DamageCauser))

(fn ConstructionScript
  (|CallParentFunction))