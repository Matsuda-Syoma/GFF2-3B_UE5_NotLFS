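; Enemy Blueprint that moves vertically by driving its CharacterMovement velocity from a timeline.
; On BeginPlay, after the parent logic, the timeline starts with its play rate set to MoveSpeed.
; Each update sets Z velocity from the MoveY track, scaled by frame delta time, MoveSpeed, MoveLength and a constant, with X and Y zeroed.
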(event EventBeginPlay
  (|CallParentFunction)
  (Components|Timeline|SetPlayRate (Variables|Default|Getタイムライン) (Variables|Default|GetMoveSpeed))
  (bind _movey (Timeline|タイムライン PlayFromStart)
    (:Update
      (Variables|/Script/Engine.MovementComponent|SetVelocity (Variables|Character|GetCharacterMovement) (Math|Vector|MakeVector 0.0 0.0 (* (* (Utilities|Time|GetWorldDeltaSeconds) _movey) (* (Variables|Default|GetMoveSpeed) 1e+04 (Variables|Default|GetMoveLength))))))))

(fn ConstructionScript
  (|CallParentFunction))