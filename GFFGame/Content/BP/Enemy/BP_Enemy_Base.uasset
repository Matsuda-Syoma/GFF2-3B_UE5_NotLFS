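; Base Paper2D enemy character with flipbook animation, health, a widget HP bar and score drops on death.
; Damage updates the bar and a delayed lerped delta bar, with a scale hit reaction and timed bar hiding.
; On death it randomly picks a count up to twenty that evenly divides its score, spawns that many score-carrying actors, credits the GameMode, then runs a death effect and destroys itself.
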(event Custom|DeathEvent
  (CallFunction|GetTex (Variables|Default|GetTexture) self "0.000000,1.000000,-20.000000" 1.0 (Variables|Default|GetReverse?))
  (Actor|DestroyActor))

(event Game|Damage|EventAnyDamage
  (params (Damage :type Float%20%28single-precision%29) (DamageType :type Damage%20Type%20Object%20Reference) (InstigatedBy :type Controller%20Object%20Reference) (DamageCauser :type Actor%20Object%20Reference))
  (bind _randnum (Variables|Default|GetRandNum))
  (bind (_outitem _outindex) (Utilities|Array|Random _randnum))
  (|Damage Damage)
  (if (CallFunction|DeathCheck)
    (if (not (Variables|Default|Getdeath))
      (Audio|PlaySound2D 0 1.0 1.0 0.0 0 0)
      (Variables|Default|Setdeath true)
      (CallFunction|DeathEvent)
      (bind _output_get (Variables|Default|SetNewVar 20))
      (for _index (range 1 _output_get)
        (Utilities|Array|Add (Variables|Default|GetRandNum) _index))
      (Variables|Default|SetDropScoreNum _outitem :!label _label)
      (if (== (Math|Integer|%(Integer) (Variables|STATE|GetSTATE_SCORE) (Variables|Default|GetDropScoreNum)) 0)
        (for _index_2 (range 1 (Variables|Default|GetDropScoreNum))
          (Game|SpawnActorfromClass "/Game/BP/NewBlueprint1.NewBlueprint1_C" (Math|Transform|MakeTransform (Transformation|GetActorLocation) "0, 0, 0" "1.000000,1.000000,1.000000") "Undefined" "MultiplyWithRoot" 0 (Math|Float|Truncate (/ (Variables|STATE|GetSTATE_SCORE) (Variables|Default|GetDropScoreNum))) 0))
        (Default|AddDataScore (CallFunction|GetGameMode) (Variables|STATE|GetSTATE_SCORE))
        (Utilities|Array|Clear (Variables|Default|GetRandNum))
        (else
          (Utilities|Array|RemoveIndex (Variables|Default|GetRandNum) _outindex)
          (goto _label))))
    (else
      (Rendering|SetVisibility (Variables|Default|GetHPBar) true false)
      (bind _color (Timeline|HitViewSize PlayFromStart)
        (:Update
          (Transformation|SetRelativeScale3D (Variables|Default|GetSprite) (Math|Conversions|ToVector(Float) _color))
          (Utilities|FlowControl|RetriggerableDelay 2.0)
          (Rendering|SetVisibility (Variables|Default|GetHPBar) false false))))))

(event EventTick
  (params (DeltaSeconds :type Float%20%28single-precision%29))
  (CallFunction|EnemyAnimation)
  (if (Variables|Default|Getdeath)
    (Collision|SetCollisionProfileName (Variables|Collision|GetCapsuleComponent) "OverlapOnlyPawn" true :!class /Script/Engine.PrimitiveComponent)))

(event EventBeginPlay
  (CallFunction|LoadWidget)
  (DataTable|GetDataTableRowNames "/Game/BP/Enemy/DT_Type.DT_Type"))

(fn ConstructionScript
  (bind _output_get (Variables|VALUE|SetVALUE_HP (Math|Conversions|ToFloat(Integer) (Variables|STATE|GetSTATE_HP))))
  (Variables|VALUE|SetVALUE_DELTAHP _output_get)
  (Variables|VALUE|SetVALUE_DAMAGE (Variables|STATE|GetSTATE_DAMAGE))
  (Variables|VALUE|SetVALUE_SCORE (Variables|STATE|GetSTATE_SCORE)))

(fn SetDamage
  (params (Damage :type Float%20%28double-precision%29))
  (bind _output_get (Variables|VALUE|SetVALUE_HP (- (Variables|VALUE|GetVALUE_HP) Damage)))
  (return _output_get))

(fn DeathCheck
  (return (<= (Variables|VALUE|GetVALUE_HP) 0.0)))

(fn LoadWidget
  (bind _asui_enemy_hp (Utilities|Casting|CastToUI_EnemyHP (UserInterface|GetUserWidgetObject (Variables|Default|GetHPBar))))
  (Variables|Default|SetAs%20UI%20Enemy%20HP _asui_enemy_hp))

(fn EnemyAnimation
  (Components|Timeline|SetLooping (Variables|Default|GetSprite) true)
  (Audio|Components|Audio|Play (Variables|Default|GetSprite))
  (if (AI|Components|NavMovement|IsFalling (Variables|Character|GetCharacterMovement))
    (Sprite|SetFlipbook (Variables|Default|GetSprite) (Variables|Default|GetAnim_Jump))
    (Components|Timeline|SetLooping (Variables|Default|GetSprite) false)
    (elif (Variables|Default|Getdeath)
      (Sprite|SetFlipbook (Variables|Default|GetSprite) (Variables|Default|GetAnim_Dead))
      (Components|Timeline|SetLooping (Variables|Default|GetSprite) false)
      (elif (!= (.x (Transformation|GetVelocity)) 0.0)
        (Sprite|SetFlipbook (Variables|Default|GetSprite) (Variables|Default|GetAnim_Run))
        (else
          (Sprite|SetFlipbook (Variables|Default|GetSprite) (Variables|Default|GetAnim_Stay)))))))