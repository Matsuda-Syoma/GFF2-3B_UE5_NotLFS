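; BP_Enemy_Vulture is a 2D vulture enemy that inherits from a parent enemy Blueprint.
; BeginPlay and the construction script only call the parent, and Tick and overlap events are disabled stubs.
; EnemyAnimation selects the sprite flipbook from movement and death state: jump while falling, otherwise dead, run or stay.
; Falling takes priority over death, and only the death flipbook plays without looping.
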(event EventBeginPlay
  (|CallParentFunction))

(event Collision|EventActorBeginOverlap
  (params (OtherActor :type Actor%20Object%20Reference)))

(event EventTick
  (params (DeltaSeconds :type Float%20%28single-precision%29))
  (|CallParentFunction DeltaSeconds) ; このノードは無効になっているため呼び出せません。\n機能をビルドするにはピンをドラッグしてください。
)

(fn ConstructionScript
  (|CallParentFunction))

(fn EnemyAnimation
  (Components|Timeline|SetLooping (Variables|Default|GetSprite) true)
  (Audio|Components|Audio|Play (Variables|Default|GetSprite))
  (if (AI|Components|NavMovement|IsFalling (Variables|Character|GetCharacterMovement))
    (Sprite|SetFlipbook (Variables|Default|GetSprite) (Variables|Default|GetAnim_Jump))
    (elif (Variables|Default|Getdeath)
      (Sprite|SetFlipbook (Variables|Default|GetSprite) (Variables|Default|GetAnim_Dead))
      (Components|Timeline|SetLooping (Variables|Default|GetSprite) false)
      (elif (!= (.x (Transformation|GetVelocity)) 0.0)
        (Sprite|SetFlipbook (Variables|Default|GetSprite) (Variables|Default|GetAnim_Run))
        (else
          (Sprite|SetFlipbook (Variables|Default|GetSprite) (Variables|Default|GetAnim_Stay)))))))