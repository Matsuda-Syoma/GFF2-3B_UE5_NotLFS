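; BP_Enemy_Tarret2 is an enemy turret that continuously spawns BP_SmallAmmo projectiles from its Shot1 component's transform.
; Tick fires whenever the ShotCT flag is clear, then holds it for a Delay of frame delta times ShotCTE, so the cooldown scales with frame time.
; The live path has no aiming or range check; an unconnected branch holds unused arc-trajectory prediction toward the player.
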(event EventTick
  (params (DeltaSeconds :type Float%20%28single-precision%29))
  (bind _self self)
  (if (not (Variables|Default|GetShotCT))
    (Game|SpawnActorfromClass "/Game/BP/Ammo/BP_SmallAmmo.BP_SmallAmmo_C" (Transformation|GetSocketTransform (Variables|Default|GetShot1) "None" "RTS_World") "Undefined" "MultiplyWithRoot" 0 _self 1 _self)
    (Variables|Default|SetShotCT true)
    (Utilities|FlowControl|Delay (* (Utilities|Time|GetWorldDeltaSeconds) (Variables|Default|GetShotCT_E)))
    (Variables|Default|SetShotCT false)))

(fn ConstructionScript
  (|CallParentFunction))